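; Physics-driven VR puppet hand for BP_VRPuppetCharacter that follows a target and grabs objects.
; BeginPlay builds Physics Control controls pulling the palm and fingers toward their targets with gravity off, and configures OpenXR hand pose by side.
; BeginHold constrains the grabbed component to the hand bone, optionally offsetting throwables by GrabStyle, and flags the anim instance.
; Holds end on constraint break, teleport, or excessive palm drift from its target.
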(event `self.ReceiveBeginPlay`
  (bind _physicscontroldata (make `PhysicsControlData` 8.0 1.0 0.0 0.0 8.0 1.0 0.0 0.0 1.0 1.0 1.0 (0.0 0.0 0.0) true false false true true))
  (bind _limb_setup_data (`self.Limb Setup Data`))
  (bind _isright (`self.IsRight`))
  (bind _physicscontrol (`self.PhysicsControl`))
  (bind _handmesh (`self.HandMesh`))
  (bind (_returnvalue_location _returnvalue_rotation) (`KismetMathLibrary.BreakTransform` (`SkinnedMeshComponent.GetBoneTransform` _handmesh "hand_r" "RTS_World")))
  (`|ExecutionSequence`
    (:`then_0`
      (`SceneComponent.K2_SetWorldTransform` (`self.TargetRoot`) (`KismetMathLibrary.MakeTransform` (`PrimitiveComponent.GetCenterOfMass` _handmesh "hand_r") _returnvalue_rotation) false true))
    (:`then_1`
      (for (_ _array_index) _limb_setup_data
        (setmembers `PhysicsControlLimbSetupData` :`StructRef` (`|GetArrayItem` _limb_setup_data _array_index) :`bCreateWorldSpaceControls` (`.bEnabled` (break `PhysicsControlData` (`self.FingerBonesWorldSpaceControlData`))) :`bCreateParentSpaceControls` (`.bEnabled` (break `PhysicsControlData` (`self.FingerBonesParentSpaceControlData`))))))
    (:`then_2`
      (bind (_allworldspacecontrols _limbworldspacecontrols _allparentspacecontrols _limbparentspacecontrols _allbodymodifiers) (`PhysicsControlComponent.CreateControlsAndBodyModifiersFromLimbBones` (`self.PhysicsControl`) (`self.HandMesh`) (`self.Limb Setup Data`) (`self.FingerBonesWorldSpaceControlData`) (`self.FingerBonesParentSpaceControlData`) (make `PhysicsControlModifierData` "Simulated" "QueryAndPhysics" 0.0) (`self.HandTarget`) "None"))
      (set `self.All Body Modifiers` _allbodymodifiers)
      (set `self.PalmOpenControlData` _physicscontroldata)
      (`PhysicsControlComponent.CreateNamedControl` :`self` _physicscontrol :`Name` "palm" :`ParentMeshComponent` (`self.HandTarget`) :`ChildMeshComponent` (`self.HandMesh`) :`ChildBoneName` "hand_r" :`ControlData` _physicscontroldata)
      (`PhysicsControlComponent.CreateNamedBodyModifier` _physicscontrol "palm" null "hand_r" "None" (make `PhysicsControlModifierData` "Simulated" "PhysicsOnly" 0.0 1.0 false false)))
    (:`then_3`
      (bind _asbp_vrpuppet_character (cast `/Game/Puppet/Character/BP_VRPuppetCharacter` (`self.GetOwner`)))
      (bind _output_get (set `self.OwningCharacter` _asbp_vrpuppet_character))
      (`self.BindEvents` _output_get))
    (:`then_4`
      (setmembers `BPOpenXRActionSkeletalData` :`StructRef` (`|GetArrayItem` (`OpenXRHandPoseComponent.HandSkeletalActions` (`self.OpenXRHandPose`))) :`TargetHand` (select `bool` _isright :`false` "EActionHandIndex_Left" :`true` "EActionHandIndex_Right" :!type "EVRSkeletalHandIndex Enum") :`bMirrorLeftRight` (not _isright)))))

(event `BeginHold`
  (params (GrabbedComponent :type "PrimitiveComponent Object Reference"))
  (bind _interactableconstraint (`self.InteractableConstraint`))
  (bind (_outpointonbody _returnvalue) (`PrimitiveComponent.GetClosestPointOnCollision` GrabbedComponent (`SceneComponent.K2_GetComponentLocation` (`self.GrabSphere`)) "None"))
  (`/Engine/EditorBlueprintResources/StandardMacros.IsValid` GrabbedComponent
    (:`Is Valid`
      (bind _asbp_throwable_actor (cast `/Game/Puppet/Interactables/BP_ThrowableActor` (`ActorComponent.GetOwner` GrabbedComponent))
        (:`then`
          (switch `/Game/Puppet/PuppetGrabStyle` (`/Game/Puppet/Interactables/BP_ThrowableActor.GrabStyle` _asbp_throwable_actor)
            (:`NewEnumerator0`
              _)
            (:`NewEnumerator1`
              (if (> _returnvalue 0.0) :!label _label
                (`PhysicsConstraintComponent.SetLinearPositionTarget` _interactableconstraint (* (`KismetMathLibrary.GetDirectionUnitVector` _outpointonbody) _returnvalue))))))
        (:`CastFailed`
          (bind _asbp_throwable_component (cast `/Game/Puppet/Interactables/BP_ThrowableComponent` GrabbedComponent)
            (:`then`
              (switch `/Game/Puppet/PuppetGrabStyle` (`/Game/Puppet/Interactables/BP_ThrowableComponent.GrabStyle` _asbp_throwable_component)
                (:`NewEnumerator0`
                  _)
                (:`NewEnumerator1`
                  (goto _label))))
            (:`CastFailed`
              _))))
      (`PhysicsConstraintComponent.SetConstrainedComponents` _interactableconstraint GrabbedComponent "None" (`self.HandMesh`) "hand_r")
      (bind _asabp_puppet_hand (cast `/Game/Puppet/ABP_PuppetHand` (`SkeletalMeshComponent.GetAnimInstance` (`self.HandMesh`))))
      (set `/Game/Puppet/ABP_PuppetHand.IsGrabbing` true _asabp_puppet_hand))
    (:`Is Not Valid`
      (`KismetSystemLibrary.PrintString` "[PuppetHand] FAIL: Grabbed object is not a PrimitiveComponent" true true (struct :`R` 1.0 :`G` 0.103638 :`B` 0.09369 :`A` 1.0)))))

(event `self.ReceiveTick`
  (params (DeltaSeconds :type "Float (single-precision)"))
  (bind _returnvalue_location (`KismetMathLibrary.BreakTransform` (`KismetMathLibrary.MakeRelativeTransform` (`PhysicsObjectBlueprintLibrary.GetPhysicsObjectWorldTransform` (`self.HandMesh`) "hand_r") (`PhysicsObjectBlueprintLibrary.GetPhysicsObjectWorldTransform` (`self.HandTarget`)))))
  (if (>= (`KismetMathLibrary.Vector_Distance` _returnvalue_location) 25.0)
    (`self.EndHold`)))

(event `EndHold`
  (`PhysicsConstraintComponent.BreakConstraint` (`self.InteractableConstraint`))
  (bind _asabp_puppet_hand (cast `/Game/Puppet/ABP_PuppetHand` (`SkeletalMeshComponent.GetAnimInstance` (`self.HandMesh`))))
  (set `/Game/Puppet/ABP_PuppetHand.IsGrabbing` false _asabp_puppet_hand))

(event `self.InteractableConstraint.OnConstraintBroken`
  (params (ConstraintIndex :type Integer))
  (`self.EndHold`))

(event `OnTeleported`
  (`/Engine/EditorBlueprintResources/StandardMacros.IsValid` (`self.AttachedInteractable`)
    (:`Is Valid`
      (`self.EndHold`))
    (:`Is Not Valid`
      _))
  (`KismetSystemLibrary.Delay` 0.0))

(fn `BindEvents`
  (params (OwningCharacter :type "/Game/Puppet/Character/BP_VRPuppetCharacter Object Reference"))
  (if (and (`KismetSystemLibrary.IsValid` (`self.OtherController`)) (`KismetSystemLibrary.IsValid` (`self.OwnerController`)))
    (add `VRBaseCharacter.OnCharacterTeleported_Bind` OwningCharacter (`|CreateDelegate` :!event `OnTeleported`))))

(fn `UserConstructionScript`)