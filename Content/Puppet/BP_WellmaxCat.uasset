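; Physics-driven cat puppet that configures its skeletal mesh for Physics Control on BeginPlay.
; Creates world-space controls, parent-space controls and body modifiers from limb setup data, then stores the results in variables via a collapsed graph.
; Groups whisker and ear modifiers into named sets, partially blends physics on the whiskers, disables parent-space controls and makes the root kinematic.
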(event `self.ReceiveBeginPlay`
  (bind (_allworldspacecontrols _limbworldspacecontrols _allparentspacecontrols _limbparentspacecontrols _allbodymodifiers _limbbodymodifiers) (`PhysicsControlComponent.CreateControlsAndBodyModifiersFromLimbBones` (`self.PhysicsControl`) (`self.Cat`) (`self.Limb Setup Data`) (`self.World Space Control Data`) (`self.Parent Space Control Data`) (`self.Body Modifier Data`) null "None"))
  (set `self.All World Space Controls` _allworldspacecontrols)
  (set `self.Limb World Space Controls` _limbworldspacecontrols)
  (set `self.All Parent Space Controls` _allparentspacecontrols)
  (set `self.Limb Parent Space Controls` _limbparentspacecontrols)
  (set `self.All Body Modifiers` _allbodymodifiers)
  (set `self.Limb Body Modifiers` _limbbodymodifiers)
  (`|ExecutionSequence`
    (:`then_0`
      (`PhysicsControlComponent.AddBodyModifierToSet` (`self.PhysicsControl`) "whisker_l" "Whiskers")
      (`PhysicsControlComponent.AddBodyModifierToSet` (`self.PhysicsControl`) "whisker_r" "Whiskers")
      (`PhysicsControlComponent.AddBodyModifierToSet` (`self.PhysicsControl`) "ear_l" "Ears")
      (`PhysicsControlComponent.AddBodyModifierToSet` (`self.PhysicsControl`) "ear_r" "Ears"))
    (:`then_1`
      (`PhysicsControlComponent.SetBodyModifiersInSetPhysicsBlendWeight` (`self.PhysicsControl`) "Whiskers" 0.25))
    (:`then_2`
      (`PhysicsControlComponent.SetControlsInSetEnabled` (`self.PhysicsControl`) "ParentSpace" false)
      (`PhysicsControlComponent.SetBodyModifierMovementType` (`self.PhysicsControl`) "root" "Kinematic"))))

(fn `UserConstructionScript`)