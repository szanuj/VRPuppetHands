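; BP_Door is an interactable physics door that latches shut and releases when its handle is turned.
; Each tick, it enables physics on Door once the Handles pitch passes a threshold derived from HandleConstraint's Swing2 limit.
; It disables physics once the door's yaw relative to Frame is zero or below and the handle is released.
; That yaw comes from world transforms, because a simulated component's relative transform ignores the component hierarchy.
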(event `self.ReceiveTick`
  (params (DeltaSeconds :type "Float (single-precision)"))
  (bind (_relativerotation_roll _relativerotation_pitch) (`KismetMathLibrary.BreakRotator` (`SceneComponent.RelativeRotation` (`self.Handles`))))
  (bind _returnvalue (<= _relativerotation_pitch (* (`.Swing2Limit` (`VREPhysicsConstraintComponent.GetAngularLimits` (`self.HandleConstraint`))) -2.0)))
  (if (`SceneComponent.IsSimulatingPhysics` (`self.Door`) "None")
    (if (and (<= (.yaw (.rotation (`KismetMathLibrary.MakeRelativeTransform` (`SceneComponent.K2_GetComponentToWorld` (`self.Door`)) (`SceneComponent.K2_GetComponentToWorld` (`self.Frame`))))) 0.0) (not _returnvalue))
      (`PrimitiveComponent.SetSimulatePhysics` (`self.Door`) false))
    (elif _returnvalue
      (`PrimitiveComponent.SetSimulatePhysics` (`self.Door`) true))))

(fn `UserConstructionScript`)