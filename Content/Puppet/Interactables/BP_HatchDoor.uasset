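; BP_HatchDoor is an interactable hatch with two door halves that slide apart according to the value of its Mechanism.
; UpdateDoors runs on BeginPlay and whenever the Mechanism value changes, so the doors follow that value directly, with no timeline or tick.
; It maps the value linearly to a local Y offset, mirrored between DoorL and DoorR, without clamping.
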(event `self.ReceiveBeginPlay`
  (`self.UpdateDoors` :!label _label))

(event `self.Mechanism.OnValueChanged`
  (params (Delta :type "Float (double-precision)"))
  (goto _label))

(event `UpdateDoors`
  (bind _returnvalue (`KismetMathLibrary.MapRangeUnclamped` (`/Game/Puppet/Interactables/BP_Mechanism.Value` (`self.Mechanism`)) 0.0 1.0 0.0 45.0))
  (`SceneComponent.K2_SetRelativeLocation` (`self.Door_r`) (`KismetMathLibrary.MakeVector` 0.0 (* _returnvalue -1.0)) false false)
  (`SceneComponent.K2_SetRelativeLocation` (`self.Door_l`) (`KismetMathLibrary.MakeVector` 0.0 _returnvalue) false false))

(fn `UserConstructionScript`)