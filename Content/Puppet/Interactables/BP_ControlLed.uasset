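; BP_ControlLed is an LED indicator whose glow and point light brightness follow the value of a Mechanism.
; On BeginPlay it creates a dynamic material, stores maximum light intensity and emissive color, and applies an optional hue override.
; Each value change scales light intensity and emissive HSV value from those maxima.
; Tick watches for Hue changes while override is on, re-tinting material and light while keeping saturation and brightness.
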(event `self.ReceiveBeginPlay`
  (bind _emissivecolorcurrent (`self.EmissiveColorCurrent`))
  (bind _pointlight (`self.PointLight`))
  (bind _ledmaterialinstance (`self.LedMaterialInstance`))
  (bind (_returnvalue_r _returnvalue_g _returnvalue_b _returnvalue_a) (break `LinearColor` (`KismetMathLibrary.RGBLinearToHSV` (`LightComponentBase.GetLightColor` _pointlight))))
  (set `self.LightIntensityMax` (`LightComponentBase.Intensity` (`self.PointLight`)))
  (bind _returnvalue (`PrimitiveComponent.CreateDynamicMaterialInstance` (`self.Led`) 0 null "None"))
  (bind _output_get (set `self.LedMaterialInstance` _returnvalue))
  (bind _returnvalue_2 (`MaterialInstanceDynamic.K2_GetVectorParameterValue` _output_get "Emissive"))
  (bind (_returnvalue_r_2 _returnvalue_g_2 _returnvalue_b_2 _returnvalue_a_2) (break `LinearColor` (`KismetMathLibrary.RGBLinearToHSV` _returnvalue_2)))
  (`KismetMathLibrary.LinearColor_SetFromHSV` _emissivecolorcurrent (`KismetMathLibrary.SelectFloat` (`self.Hue`) _returnvalue_r_2 (`self.OverrideHue`)) _returnvalue_g_2 _returnvalue_b_2 _returnvalue_a_2)
  (set `self.EmissiveColorMax` _emissivecolorcurrent)
  (bind _returnvalue_3 (`MaterialInstanceDynamic.K2_GetVectorParameterValue` _ledmaterialinstance "Color"))
  (bind (_returnvalue_r_3 _returnvalue_g_3 _returnvalue_b_3 _returnvalue_a_3) (break `LinearColor` (`KismetMathLibrary.RGBLinearToHSV` _returnvalue_3)))
  (`MaterialInstanceDynamic.SetVectorParameterValue` _ledmaterialinstance "Color" (`KismetMathLibrary.HSVToRGBLinear` (make `LinearColor` (`KismetMathLibrary.SelectFloat` (`self.Hue`) _returnvalue_r_3 (`self.OverrideHue`)) _returnvalue_g_3 _returnvalue_b_3 _returnvalue_a_3)))
  (`LightComponent.SetLightColor` _pointlight (`KismetMathLibrary.HSVToRGBLinear` (make `LinearColor` (`KismetMathLibrary.SelectFloat` (`self.Hue`) _returnvalue_r (`self.OverrideHue`)) _returnvalue_g _returnvalue_b _returnvalue_a)) true)
  (`self.UpdateLed`))

(event `self.Mechanism.OnValueChanged`
  (params (Delta :type "Float (double-precision)"))
  (`self.UpdateLed`))

(event `UpdateLed`
  (bind _emissivecolorcurrent (`self.EmissiveColorCurrent`))
  (bind (_returnvalue_r _returnvalue_g _returnvalue_b _returnvalue_a) (break `LinearColor` (`KismetMathLibrary.RGBLinearToHSV` (`self.EmissiveColorMax`))))
  (bind (_returnvalue_r_2 _returnvalue_g_2 _returnvalue_b_2) (break `LinearColor` (`KismetMathLibrary.RGBLinearToHSV` (`self.EmissiveColorMax`))))
  (bind _value (`/Game/Puppet/Interactables/BP_Mechanism.Value` (`self.Mechanism`)))
  (`LightComponent.SetIntensity` (`self.PointLight`) (`KismetMathLibrary.MapRangeUnclamped` _value 0.0 1.0 0.0 (`self.LightIntensityMax`)))
  (`KismetMathLibrary.LinearColor_SetFromHSV` _emissivecolorcurrent _returnvalue_r _returnvalue_g (`KismetMathLibrary.MapRangeUnclamped` _value 0.0 1.0 0.0 _returnvalue_b_2) _returnvalue_a)
  (`MaterialInstanceDynamic.SetVectorParameterValue` (`self.LedMaterialInstance`) "Emissive" _emissivecolorcurrent))

(event `self.ReceiveTick`
  (params (DeltaSeconds :type "Float (single-precision)"))
  (`self.CheckUpdateHue`))

(fn `CheckUpdateHue`
  (bind _ledmaterialinstance (`self.LedMaterialInstance`))
  (bind _emissivecolorcurrent (`self.EmissiveColorCurrent`))
  (bind _pointlight (`self.PointLight`))
  (bind (_returnvalue_r _returnvalue_g _returnvalue_b _returnvalue_a) (break `LinearColor` (`KismetMathLibrary.RGBLinearToHSV` (`self.EmissiveColorMax`))))
  (bind (_returnvalue_r_2 _returnvalue_g_2 _returnvalue_b_2 _returnvalue_a_2) (break `LinearColor` (`KismetMathLibrary.RGBLinearToHSV` (`self.EmissiveColorCurrent`))))
  (bind (_returnvalue_r_3 _returnvalue_g_3 _returnvalue_b_3 _returnvalue_a_3) (break `LinearColor` (`KismetMathLibrary.RGBLinearToHSV` (`LightComponentBase.GetLightColor` _pointlight))))
  (if (and (`self.OverrideHue`) (> (`KismetMathLibrary.Abs` (- (`self.Hue`) _returnvalue_r)) 0.01))
    (`KismetMathLibrary.LinearColor_SetFromHSV` (`self.EmissiveColorMax`) (`self.Hue`) _returnvalue_g _returnvalue_b _returnvalue_a)
    (`KismetMathLibrary.LinearColor_SetFromHSV` _emissivecolorcurrent (`self.Hue`) _returnvalue_g_2 _returnvalue_b_2 _returnvalue_a_2)
    (`MaterialInstanceDynamic.SetVectorParameterValue` _ledmaterialinstance "Emissive" _emissivecolorcurrent)
    (bind _returnvalue (`MaterialInstanceDynamic.K2_GetVectorParameterValue` _ledmaterialinstance "Color"))
    (bind (_returnvalue_r_4 _returnvalue_g_4 _returnvalue_b_4 _returnvalue_a_4) (break `LinearColor` (`KismetMathLibrary.RGBLinearToHSV` _returnvalue)))
    (`MaterialInstanceDynamic.SetVectorParameterValue` _ledmaterialinstance "Color" (`KismetMathLibrary.HSVToRGBLinear` (make `LinearColor` (`self.Hue`) _returnvalue_g_4 _returnvalue_b_4 _returnvalue_a_4)))
    (`LightComponent.SetLightColor` _pointlight (`KismetMathLibrary.HSVToRGBLinear` (make `LinearColor` (`self.Hue`) _returnvalue_g_3 _returnvalue_b_3 _returnvalue_a_3)) true)))

(fn `UserConstructionScript`)