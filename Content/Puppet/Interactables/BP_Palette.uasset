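; BP_Palette is an interactable paint palette that feeds colours to a BP_Paintbrush.
; On BeginPlay it binds overlap events on each primitive child of the Palette component and caches that child's material "Color" parameter in a map keyed by component.
; A brush entering a mapped component begins mixing paint with the stored colour, and leaving ends the mixing.
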(event `self.ReceiveBeginPlay`
  (for _array_element (`SceneComponent.GetChildrenComponents` (`self.Palette`) false)
    (bind _asprimitive_component (cast `PrimitiveComponent` _array_element))
    (add `PrimitiveComponent.OnComponentBeginOverlap` _asprimitive_component (delegate `BrushBeginOverlap`))
    (add `PrimitiveComponent.OnComponentEndOverlap` _asprimitive_component (delegate `BrushEndOverlap`))
    (bind _returnvalue (`PrimitiveComponent.CreateDynamicMaterialInstance` _asprimitive_component 0 (`PrimitiveComponent.GetMaterial` _asprimitive_component 0) "None"))
    (bind _returnvalue_2 (`MaterialInstanceDynamic.K2_GetVectorParameterValue` _returnvalue "Color"))
    (`BlueprintMapLibrary.Map_Add` (`self.ColorMap`) _asprimitive_component _returnvalue_2)))

(event `BrushBeginOverlap`
  (params (OverlappedComponent :type "PrimitiveComponent Object Reference") (OtherActor :type "Actor Object Reference") (OtherComp :type "PrimitiveComponent Object Reference") (OtherBodyIndex :type Integer) (bFromSweep :type Boolean) (SweepResult :type "HitResult Structure (by ref)"))
  (bind (_value _returnvalue) (`BlueprintMapLibrary.Map_Find` (`self.ColorMap`) OverlappedComponent))
  (bind _asbp_paintbrush (cast `/Game/Puppet/Interactables/BP_Paintbrush` OtherActor))
  (if _returnvalue
    (`/Game/Puppet/Interactables/BP_Paintbrush.BeginMixingPaint` _asbp_paintbrush _value)))

(event `BrushEndOverlap`
  (params (OverlappedComponent :type "PrimitiveComponent Object Reference") (OtherActor :type "Actor Object Reference") (OtherComp :type "PrimitiveComponent Object Reference") (OtherBodyIndex :type Integer))
  (bind _asbp_paintbrush (cast `/Game/Puppet/Interactables/BP_Paintbrush` OtherActor))
  (`/Game/Puppet/Interactables/BP_Paintbrush.EndMixingPaint` _asbp_paintbrush))

(fn `UserConstructionScript`)