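; Base grippable tool for interacting with a BP_Canvas, leaving InitInteraction and PerformInteraction empty for child tools to implement.
; Enable and disable checks track the canvas from objects passed to them.
; For the locally controlled gripper, gripping or acquiring a canvas starts a looping PerformInteraction timer, cleared on release or canvas loss.
; A helper converts world locations to canvas UVs through the canvas.
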(event `self.ReceiveBeginPlay`)

(event `VRGripInterface.OnGrip`
  (params (GrippingController :type "GripMotionControllerComponent Object Reference") (GripInformation :type "BPActorGripInformation Structure (by ref)"))
  (bind _returnvalue (`GripMotionControllerComponent.BP_IsLocallyControlled` GrippingController))
  (`parent.OnGrip` GrippingController GripInformation)
  (set `self.bIsLocalTool` _returnvalue)
  (if (and (`KismetSystemLibrary.IsValid` (`self.CanvasInteractable`)) (not (`KismetSystemLibrary.K2_IsValidTimerHandle` (`self.InteractionTimer`))))
    (if _returnvalue
      (bind _returnvalue_2 (`KismetSystemLibrary.K2_SetTimer` self "PerformInteraction" (`self.InteractionRate`) true))
      (set `self.InteractionTimer` _returnvalue_2)
      (`self.InitInteraction`))))

(event `VRGripInterface.OnGripRelease`
  (params (ReleasingController :type "GripMotionControllerComponent Object Reference") (GripInformation :type "BPActorGripInformation Structure (by ref)") (bWasSocketed :type Boolean))
  (bind _interactiontimer (`self.InteractionTimer`))
  (`parent.OnGripRelease` ReleasingController GripInformation bWasSocketed)
  (if (`KismetSystemLibrary.K2_IsValidTimerHandle` _interactiontimer)
    (`KismetSystemLibrary.K2_ClearAndInvalidateTimerHandle` _interactiontimer)))

(fn `CalcRelativePositionToCanvas`
  (params (WorldLocation :type "Vector Structure"))
  (returns (HitLoc :type "Vector2D Structure"))
  (bind _canvasinteractable (`self.CanvasInteractable`))
  (`/Engine/EditorBlueprintResources/StandardMacros.IsValid` _canvasinteractable
    (:`Is Valid`
      (bind _hitloc (`/Game/Puppet/Interactables/BP_Canvas.CalcRelativePos` _canvasinteractable WorldLocation))
      (return _hitloc) ; Hit Loc In UV
    )
    (:`Is Not Valid`
      (return (0.0 0.0)) ; Hit Loc In UV
    )))

(fn `CheckDisableInteractionWithCanvas`
  (params (Object :type "Object Object Reference"))
  (bind _canvasinteractable (`self.CanvasInteractable`))
  (`/Engine/EditorBlueprintResources/StandardMacros.IsValid` _canvasinteractable
    (:`Is Valid`
      (if (== Object _canvasinteractable)
        (set `self.CanvasInteractable` null)
        (`KismetSystemLibrary.K2_ClearAndInvalidateTimerHandle` (`self.InteractionTimer`))))))

(fn `CheckEnableInteractionWithCanvas`
  (params (Overlap :type "Object Object Reference"))
  (`/Engine/EditorBlueprintResources/StandardMacros.IsValid` Overlap
    (:`Is Valid`
      (if (and (not (`KismetSystemLibrary.IsValid` (`self.CanvasInteractable`))) (`KismetMathLibrary.ClassIsChildOf` (`GameplayStatics.GetObjectClass` Overlap) "/Game/Puppet/Interactables/BP_Canvas.BP_Canvas_C"))
        (bind _asbp_canvas (cast `/Game/Puppet/Interactables/BP_Canvas` Overlap))
        (set `self.CanvasInteractable` _asbp_canvas)
        (if (`self.bIsLocalTool`)
          (bind _returnvalue (`KismetSystemLibrary.K2_SetTimer` self "PerformInteraction" (`self.InteractionRate`) true))
          (set `self.InteractionTimer` _returnvalue)
          (`self.InitInteraction`))))))

(fn `InitInteraction`)

(fn `PerformInteraction`)

(fn `UserConstructionScript`)