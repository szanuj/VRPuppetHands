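; BP_Slider is a puppet interactable slider that reports its position as a normalized value.
; On BeginPlay it sets the reference position of the Rail physics constraint's first frame.
; GetValues takes the Slider's Y location relative to Base and maps the Rail's symmetric linear limits to an inverted, clamped 1-to-0 range.
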(event `self.ReceiveBeginPlay`
  (`parent.ReceiveBeginPlay`)
  (`PhysicsConstraintComponent.SetConstraintReferencePosition` (`self.Rail`) "Frame1" (0.0 0.0 0.0)))

(fn `GetValues`
  (returns (Value :type "Float (double-precision)"))
  (bind _linearlimit (`VREPhysicsConstraintComponent.GetLinearLimits` (`self.Rail`)))
  (return (`KismetMathLibrary.MapRangeClamped` (.y (.location (`KismetMathLibrary.MakeRelativeTransform` (`SceneComponent.K2_GetComponentToWorld` (`self.Slider`)) (`SceneComponent.K2_GetComponentToWorld` (`self.Base`))))) (* _linearlimit -1.0) _linearlimit 1.0)))

(fn `UserConstructionScript`
  (`parent.UserConstructionScript`))