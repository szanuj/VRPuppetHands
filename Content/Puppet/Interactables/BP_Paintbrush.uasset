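; VR paintbrush interactable that carries a paint color on its tip and draws on canvases.
; A tip sphere's overlaps toggle canvas interaction, which queues line segments between successive canvas-relative positions through the canvas's VRRenderTargetManager.
; A dry brush takes offered paint instantly; a loaded one blends by accumulated squared tip movement in HSV, keeping hue when mixing near-grayscale paint.
; A dynamic material shows the current color.
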(event `self.ReceiveBeginPlay`
  (bind _tip (`self.Tip`))
  (`SceneComponent.K2_AttachToComponent` (`self.Sphere`) (`self.Tip`) "tip_02" "KeepWorld" "KeepWorld" "KeepWorld" false)
  (bind _returnvalue (`PrimitiveComponent.CreateDynamicMaterialInstance` _tip 1 (`PrimitiveComponent.GetMaterial` _tip 0) "None"))
  (bind _output_get (set `self.PaintMaterial` _returnvalue))
  (bind _returnvalue_2 (`MaterialInstanceDynamic.K2_GetVectorParameterValue` _output_get "Color"))
  (bind _output_get_2 (set `self.ColorNoPaint` _returnvalue_2))
  (bind _output_get_3 (set `self.HasPaint` (`self.StartsWithPaint`)))
  (if _output_get_3
    (`self.SetPaintColor` _output_get_2)))

(event `self.ReceiveTick`
  (params (DeltaSeconds :type "Float (single-precision)"))
  (`parent.ReceiveTick` DeltaSeconds)
  (if (`self.IsMixingPaint`)
    (bind _output_get (set `self.CurrentMixingDistanceSqr` (+ (`KismetMathLibrary.Vector_DistanceSquared` (`SceneComponent.K2_GetComponentLocation` (`self.Sphere`)) (`self.LastTipLocation`)) (`self.CurrentMixingDistanceSqr`))))
    (set `self.LastTipLocation` (`SceneComponent.K2_GetComponentLocation` (`self.Sphere`)))
    (if (>= _output_get (`self.StepMixingDistanceSqr`))
      (`self.MixPaintStep` (`self.CurrentMixingDistanceSqr`))
      (set `self.CurrentMixingDistanceSqr` 0.0))))

(event `self.Sphere.OnComponentBeginOverlap`
  (params (OverlappedComponent :type "PrimitiveComponent Object Reference") (OtherActor :type "Actor Object Reference") (OtherComp :type "PrimitiveComponent Object Reference") (OtherBodyIndex :type Integer) (bFromSweep :type Boolean) (SweepResult :type "HitResult Structure (by ref)"))
  (if (`self.HasPaint`)
    (`self.CheckEnableInteractionWithCanvas` OtherActor)))

(event `self.Sphere.OnComponentEndOverlap`
  (params (OverlappedComponent :type "PrimitiveComponent Object Reference") (OtherActor :type "Actor Object Reference") (OtherComp :type "PrimitiveComponent Object Reference") (OtherBodyIndex :type Integer))
  (`self.CheckDisableInteractionWithCanvas` OtherActor))

(fn `BeginMixingPaint`
  (params (Color :type "LinearColor Structure"))
  (bind _output_get (set `self.PaintToMix` Color))
  (set `self.LastTipLocation` (`SceneComponent.K2_GetComponentLocation` (`self.Sphere`)))
  (set `self.CurrentMixingDistanceSqr` 0.0)
  (if (`self.HasPaint`)
    (set `self.IsMixingPaint` true)
    (else
      (`self.SetPaintColor` _output_get))))

(fn `ClearPaint`
  (set `self.HasPaint` false)
  (`MaterialInstanceDynamic.SetVectorParameterValue` (`self.PaintMaterial`) "Color" (`self.ColorNoPaint`)))

(fn `EndMixingPaint`
  (set `self.IsMixingPaint` false))

(fn `InitInteraction`
  (bind _hitloc (`self.CalcRelativePositionToCanvas` (`SceneComponent.K2_GetComponentLocation` (`self.Sphere`))))
  (set `self.LastHitLoc` _hitloc))

(fn `MixPaintStep`
  (params (Delta :type "Float (double-precision)"))
  (locals (IgnoreHueTolerance :type "Float (double-precision)" :default 0.01))
  (bind (_returnvalue_r _returnvalue_g _returnvalue_b _returnvalue_a) (break `LinearColor` (`KismetMathLibrary.RGBLinearToHSV` (`self.PaintToMix`))))
  (bind (_returnvalue_r_2 _returnvalue_g_2) (break `LinearColor` (`KismetMathLibrary.RGBLinearToHSV` (`self.PaintToMix`))))
  (bind (_returnvalue_r_3 _returnvalue_g_3 _returnvalue_b_2 _returnvalue_a_2) (break `LinearColor` (`KismetMathLibrary.RGBLinearToHSV` (`self.PaintColor`))))
  (bind _returnvalue (* Delta (`self.MixSpeed`)))
  (bind (_returnvalue_x _returnvalue_y _returnvalue_z) (`KismetMathLibrary.BreakVector` (`KismetMathLibrary.VLerp` (`KismetMathLibrary.MakeVector` _returnvalue_g_3 _returnvalue_b_2 _returnvalue_a_2) (`KismetMathLibrary.MakeVector` _returnvalue_g _returnvalue_b _returnvalue_a) _returnvalue)))
  (`self.SetPaintColor` (select `bool` (<= _returnvalue_g_2 (`local.IgnoreHueTolerance`)) :`false` (`KismetMathLibrary.LinearColorLerpUsingHSV` (`self.PaintColor`) (`self.PaintToMix`) _returnvalue) :`true` (`KismetMathLibrary.HSVToRGBLinear` (make `LinearColor` _returnvalue_r_3 _returnvalue_x _returnvalue_y _returnvalue_z)))))

(fn `PerformInteraction`
  (locals (ForceScaler :type "Float (double-precision)" :default 1.0))
  (bind _hitloc (`self.CalcRelativePositionToCanvas` (`SceneComponent.K2_GetComponentLocation` (`self.Sphere`))))
  (if (!= _hitloc (`self.LastHitLoc`))
    (`VRRenderTargetManager.AddLineDrawOperation` (`/Game/Puppet/Interactables/BP_Canvas.VRRenderTargetManager` (`self.CanvasInteractable`)) (`self.LastHitLoc`) _hitloc (`KismetMathLibrary.Conv_LinearColorToColor` (`self.PaintColor`) false) (`KismetMathLibrary.FTrunc` (`self.BrushThickness`)))
    (set `self.LastHitLoc` _hitloc)))

(fn `SetPaintColor`
  (params (Color :type "LinearColor Structure"))
  (bind _output_get (set `self.PaintColor` Color))
  (`MaterialInstanceDynamic.SetVectorParameterValue` (`self.PaintMaterial`) "Color" _output_get)
  (set `self.HasPaint` true)
  (return))

(fn `UserConstructionScript`
  (`parent.UserConstructionScript`))