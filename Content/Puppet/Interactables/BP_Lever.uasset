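; BP_Lever is an interactable lever that reports its position as a normalized value.
; GetValues takes the roll of the Lever relative to the Base and divides it by the Hinge constraint's twist limit.
; The result is clamped and remapped to a 0–1 range, so the center position reads as 0.5.
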(fn `GetValues`
  (returns (Value :type "Float (double-precision)"))
  (return (`KismetMathLibrary.MapRangeUnclamped` (`KismetMathLibrary.FClamp` (/ (.roll (.rotation (`KismetMathLibrary.MakeRelativeTransform` (`SceneComponent.K2_GetComponentToWorld` (`self.Lever`)) (`SceneComponent.K2_GetComponentToWorld` (`self.Base`))))) (`.TwistLimit` (`VREPhysicsConstraintComponent.GetAngularLimits` (`self.Hinge`)))) -1.0) -1.0 1.0 0.0 1.0)))

(fn `UserConstructionScript`)