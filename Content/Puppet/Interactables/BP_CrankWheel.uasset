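; BP_CrankWheel is a physics-constrained crank interactable that turns wheel rotation into a normalized 0–1 value.
; GetValues accumulates per-update roll deltas and divides the sum by AngularLimit, allowing multi-turn cranks.
; Limits under a full turn use a fixed twist constraint on CrankJoint.
; For larger limits, ValueChanged frees the joint mid-range and re-limits it near either end, offset by the wheel's current roll.
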(event `self.ReceiveBeginPlay`
  (bind _crankjoint (`self.CrankJoint`))
  (bind _crankjoint_2 (`self.CrankJoint`))
  (bind _limitactivationthreshold (`self.LimitActivationThreshold`))
  (bind _returnvalue (/ (`self.AngularLimit`) 2.0))
  (set `self.PreviousRotation` (`SceneComponent.RelativeRotation` (`self.Wheel`)))
  (`parent.ReceiveBeginPlay`)
  (if (< (`self.AngularLimit`) 360.0)
    (`PhysicsConstraintComponent.SetAngularTwistLimit` _crankjoint_2 "ACM_Limited" _returnvalue)
    (`VREPhysicsConstraintComponent.SetAngularOffset` _crankjoint_2 (`KismetMathLibrary.MakeRotator` (* _returnvalue -1.0)))
    (else
      (`PhysicsConstraintComponent.SetAngularTwistLimit` _crankjoint "ACM_Limited" _limitactivationthreshold)
      (`VREPhysicsConstraintComponent.SetAngularOffset` _crankjoint (`KismetMathLibrary.MakeRotator` (* _limitactivationthreshold -1.0))))))

(event `self.ValueChanged`
  (params (Delta :type "Float (double-precision)"))
  (bind _value (`self.Value`))
  (bind _limitactivationthreshold (`self.LimitActivationThreshold`))
  (bind _crankjoint (`self.CrankJoint`))
  (bind _crankjoint_2 (`self.CrankJoint`))
  (bind _angularlimit (`self.AngularLimit`))
  (bind _relativerotation_roll (`KismetMathLibrary.BreakRotator` (`SceneComponent.RelativeRotation` (`self.Wheel`))))
  (`parent.ValueChanged` Delta)
  ;[0.02 0.01 0.01] Handle constraint when we want more than one full spin
  (if (>= (`self.AngularLimit`) 360.0)
    (if (or (>= _value (/ (- _angularlimit _limitactivationthreshold) _angularlimit)) (<= _value (/ _limitactivationthreshold _angularlimit)))
      (if (not (`self.IsLimitActive`))
        (set `self.IsLimitActive` true)
        (`PhysicsConstraintComponent.SetAngularTwistLimit` _crankjoint "ACM_Limited" (`self.LimitActivationThreshold`))
        (`VREPhysicsConstraintComponent.SetAngularOffset` _crankjoint (`KismetMathLibrary.MakeRotator` _relativerotation_roll)))
      (elif (`self.IsLimitActive`)
        (set `self.IsLimitActive` false)
        (`PhysicsConstraintComponent.SetAngularTwistLimit` _crankjoint_2 "ACM_Free" 0.0)
        (`VREPhysicsConstraintComponent.SetAngularOffset` :`self` _crankjoint_2)))))

(fn `GetValues`
  (returns (Value :type "Float (double-precision)"))
  (bind _relativerotation (`SceneComponent.RelativeRotation` (`self.Wheel`)))
  (bind _returnvalue_roll (`KismetMathLibrary.BreakRotator` (`KismetMathLibrary.NormalizedDeltaRotator` _relativerotation (`self.PreviousRotation`))))
  (bind _returnvalue (+ (* _returnvalue_roll -1.0) (`self.SumRotation`)))
  (set `self.SumRotation` _returnvalue)
  (set `self.PreviousRotation` _relativerotation)
  (return (`KismetMathLibrary.FClamp` (/ _returnvalue (`self.AngularLimit`)))))

(fn `UserConstructionScript`)