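; BP_Button is an interactable physical push button that reports how far it is pressed.
; A linear constraint drive between the Base and Button components has its reference position offset along Z at BeginPlay.
; GetValues measures the Button's Z offset relative to the Base, divides its absolute value by the linear limit and returns it clamped to a 0–1 press amount.
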(event `self.ReceiveBeginPlay`
  (`parent.ReceiveBeginPlay`)
  (`PhysicsConstraintComponent.SetConstraintReferencePosition` (`self.LinearDrive`) "Frame1" (0.0 0.0 1.0)))

(fn `GetValues`
  (returns (Value :type "Float (double-precision)"))
  (return (`KismetMathLibrary.FClamp` (/ (`KismetMathLibrary.Abs` (.z (.location (`KismetMathLibrary.MakeRelativeTransform` (`SceneComponent.K2_GetComponentToWorld` (`self.Button`)) (`SceneComponent.K2_GetComponentToWorld` (`self.Base`)))))) (`VREPhysicsConstraintComponent.GetLinearLimits` (`self.LinearDrive`))))))

(fn `UserConstructionScript`
  (`parent.UserConstructionScript`))