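; BP_Mechanism is a base interactable that tracks a normalized value and raises events when it changes or reaches either limit.
; Tick polls GetValues, a placeholder returning zero that appears meant for child overrides, and fires OnValueChanged when the difference meets a threshold.
; Its own bound handler checks proximity to 0 or 1 within Epsilon, latching WasLimitReached so each limit event fires once per arrival.
; Both limit handlers are empty stubs.
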(event `self.ReceiveBeginPlay`
  (`|ExecutionSequence`
    (:`then_0`
      (add `self.OnValueChanged` (`|CreateDelegate` :!event `ValueChanged`))
      (add `self.OnUpperLimitReached` (`|CreateDelegate` :!event `UpperLimitReached`))
      (add `self.OnLowerLimitReached` (`|CreateDelegate` :!event `LowerLimitReached`)))
    (:`then_1`
      (bind _returnvalue (`self.IsAtLimit`))
      (set `self.WasLimitReached` _returnvalue))))

(event `self.ReceiveTick`
  (params (DeltaSeconds :type "Float (single-precision)"))
  (`self.Update`))

(event `LowerLimitReached`)

(event `UpperLimitReached`)

(event `ValueChanged` :!signature `self.OnValueChanged`
  (params (Delta :type "Float (double-precision)"))
  (bind _returnvalue (`self.IsAtLimit`))
  (if _returnvalue
    (if (not (`self.WasLimitReached`))
      (set `self.WasLimitReached` true)
      (if (>= (`self.Value`) 0.5)
        (`self.OnUpperLimitReached`)
        (else
          (`self.OnLowerLimitReached`))))
    (else
      (set `self.WasLimitReached` false))))

(fn `GetValues`
  (returns (Value :type "Float (double-precision)"))
  (return 0.0))

(fn `IsAtLimit`
  (returns (ReturnValue :type Boolean))
  (return (>= (`KismetMathLibrary.Abs` (- (* (`self.Value`) 2.0) 1.0)) (- 1.0 (`self.Epsilon`)))))

(fn `Update`
  (bind _value (`self.GetValues`))
  (bind _returnvalue (- _value (`self.Value`)))
  (if (>= (`KismetMathLibrary.Abs` _returnvalue) (`self.ValueChangeEventThreshold`))
    (set `self.Value` _value)
    (`self.OnValueChanged` _returnvalue)))

(fn `UserConstructionScript`)